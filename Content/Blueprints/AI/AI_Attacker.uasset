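; AI attacker character, a spider creature by its montage name, that chases the player, attacks in range and is part of a game-mode wave.
; A self-restarting AIMoveTo drives pursuit, while Tick plays the attack montage; its notify branch only prints, leaving DamagePlayer uncalled.
; At zero health it stops, credits the player's kill, leaves the wave, then sinks via a timeline before being destroyed.
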(event Custom|Move%20To%20Player
  (if (not (Variables|Default|GetDead))
    (AI|AIMoveTo self "0, 0, 0" (Game|GetPlayerCharacter 0) 5.0 false
      (:OnSuccess
        _)
      (:OnFail
        _))
    (CallFunction|MovetoPlayer)))

(event EventBeginPlay
  (CallFunction|MovetoPlayer))

(event Game|Damage|EventAnyDamage
  (params (Damage :type Float%20%28single-precision%29) (DamageType :type Damage%20Type%20Object%20Reference) (InstigatedBy :type Controller%20Object%20Reference) (DamageCauser :type Actor%20Object%20Reference))
  (bind _output_get (Variables|Default|SetHealth (Math|Float|Clamp(Float) (- (Variables|Default|GetHealth) Damage) 0.0 1e+02)))
  (if (== _output_get 0.0)
    (Variables|Actor|SetbCanBeDamaged false)
    (Variables|Default|SetDead true)
    (CallFunction|DisableCollision)
    (CallFunction|DeactivateAIMovement)
    (CallFunction|PlayDeathSFX)
    (CallFunction|StopAttackAnimation)
    (CallFunction|IncreasePlayerKills)
    (CallFunction|RemoveAttackerfromWave)
    (Utilities|FlowControl|Delay 3.0)
    (Variables|Default|SetDeath%20Fade%20Start%20Location (Transformation|GetActorLocation))
    (bind _death_fade_progress (Timeline|Death%20Fade PlayFromStart)
      (:Update
        (Transformation|SetActorLocation (Math|Vector|Lerp(Vector) (Variables|Default|GetDeath%20Fade%20Start%20Location) (- (Variables|Default|GetDeath%20Fade%20Start%20Location) "0, 0,200.000000") _death_fade_progress) false false))
      (:Finished
        (Actor|DestroyActor)))))

(event EventTick
  (params (DeltaSeconds :type Float%20%28single-precision%29))
  (if (not (Variables|Default|GetDead))
    (if (< (Transformation|GetDistanceTo (Game|GetPlayerCharacter 0)) (Variables|Default|GetAttackRange))
      (if (not (Animation|Montage|MontageIsPlaying (Components|SkeletalMesh|GetAnimInstance (Variables|Character|GetMesh)) "/Game/Characters/Enemy_Great_Spider/Animations/Montage_SpiderAttack.Montage_SpiderAttack"))
        (bind _notifyname (Animation|Montage|PlayMontage (Variables|Character|GetMesh) "/Game/Characters/Enemy_Great_Spider/Animations/Montage_SpiderAttack.Montage_SpiderAttack")
          (:OnNotifyBegin
            (if (Utilities|Name|Equal(Name) _notifyname "Damage Player")
              (Development|PrintString "Damage Player"))))))))

(fn ConstructionScript)

(fn DamagePlayer
  (Game|Damage|ApplyDamage (Game|GetPlayerCharacter 0) 25.0 0 0))

(fn RemoveAttackerfromWave
  (bind _asbp_mars_marine_game_mode (Utilities|Casting|CastToBP_MarsMarine_GameMode (Game|GetGameMode)))
  (Default|RemoveAttacker _asbp_mars_marine_game_mode self))

(fn IncreasePlayerKills
  (bind _asbp_marine (Utilities|Casting|CastToBP_Marine (Game|GetPlayerCharacter 0)))
  (Default|IncreaseKills _asbp_marine))

(fn StopAttackAnimation
  (Animation|Montage|MontageStop (Components|SkeletalMesh|GetAnimInstance (Variables|Character|GetMesh)) 0.0 "/Game/Characters/Enemy_Great_Spider/Animations/Montage_SpiderAttack.Montage_SpiderAttack"))

(fn PlayDeathSFX
  (Audio|SpawnSoundatLocation "/Game/Sounds/FoleyFlesh/Stereo/Cue_CreatureDeath.Cue_CreatureDeath" (Transformation|GetActorLocation) "0, 0, 0" 1.0 1.0 0.0 0 0))

(fn DisableCollision
  (Collision|SetCollisionEnabled (Variables|Collision|GetCapsuleComponent) "NoCollision"))

(fn DeactivateAIMovement
  (Components|Movement|StopMovementImmediately (Variables|Character|GetCharacterMovement))
  (Components|Activation|Deactivate (Variables|Character|GetCharacterMovement)))