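; BP_MissionArea is a volume that keeps the player inside the mission area, punishing them for staying outside too long.
; Ending overlap shows a W_MissionAreaWarning widget linked to the volume, reveals the SafeZone component and starts a looping one-second countdown timer.
; Re-entering removes the warning, resets the countdown and hides the zone.
; When time runs out, it damages the player, removes the widget and destroys itself.
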(event Custom|Start%20Death%20Warning
  (bind _timebeforedeath (CallFunction|DecreaseTimeBeforeDeath))
  (if (== _timebeforedeath 0)
    (Game|Damage|ApplyDamage (Game|GetPlayerCharacter 0) 1e+02 0 0)
    (Widget|RemovefromParent (Variables|Default|GetMissionWarningWidget))
    (Actor|DestroyActor)))

(event Collision|EventActorEndOverlap
  (params (OtherActor :type Actor%20Object%20Reference))
  (if (== OtherActor (Game|GetPlayerCharacter 0))
    (bind _returnvalue (UserInterface|CreateWidget "/Game/UI/Widgets/W_MissionAreaWarning.W_MissionAreaWarning_C" 0 self))
    (bind _output_get (Variables|Default|SetMissionWarningWidget _returnvalue))
    (UserInterface|Viewport|AddtoViewport _output_get 0)
    (Utilities|Time|SetTimerbyFunctionName 0 "Start Death Warning" 1.0 true)
    (CallFunction|ShowSafeZone)))

(event Collision|EventActorBeginOverlap
  (params (OtherActor :type Actor%20Object%20Reference))
  (bind _missionwarningwidget (Variables|Default|GetMissionWarningWidget))
  (if (== OtherActor (Game|GetPlayerCharacter 0))
    (Utilities|IsValid _missionwarningwidget
      (:Is%20Valid
        (Widget|RemovefromParent _missionwarningwidget)
        (Variables|Default|SetTimeBeforeDeath 5)
        (Utilities|Time|ClearTimerbyFunctionName 0 "Start Death Warning")
        (CallFunction|HideSafeZone)))))

(fn ConstructionScript)

(fn ResetTimeBeforeDeath
  (Variables|Default|SetTimeBeforeDeath 5))

(fn DecreaseTimeBeforeDeath
  (bind _result (Math|Integer|DecrementInt (Variables|Default|GetTimeBeforeDeath))
    (:%20%20
      (return _result))))

(fn ShowSafeZone
  (Development|SetHiddeninGame (Variables|Default|GetSafeZone) false false))

(fn HideSafeZone
  (Development|SetHiddeninGame (Variables|Default|GetSafeZone) true false))