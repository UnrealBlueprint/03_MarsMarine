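; Game mode for MarsMarine that runs endless, escalating waves of AI attackers.
; Each wave scales up in size, notifies UI through a dispatcher and starts music after a sound cue.
; A randomly delayed loop spawns attackers at random BP_EnemySpawner actors, holding while the live count is at its cap.
; RemoveAttacker triggers wave completion whenever the tracked list empties, fading the music and starting the next wave.
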(event Custom|Start%20New%20Wave
  (Math|Integer|IncrementInt (Variables|Default|GetCurrentWave)
    (:%20%20
      ;[1 1 1] Setup Wave
      (bind _output_get (Variables|Default|SetWaveSize (Math|Float|Round (* (Variables|Default|GetWaveSize) 1.5))))
      (Variables|Default|SetEnemiesToSpawn _output_get)
      (Variables|Default|SetMaxEnemiesAllowed 20)
      (Utilities|FlowControl|Sequence
        (:then_0
          ;[1 1 1] UI Dispatcher
          (Default|CallNewWaveStarted (Variables|Default|GetCurrentWave))
          (if (> (Variables|Default|GetEnemiesToSpawn) 0) :!label _label
            (Utilities|FlowControl|Delay (Math|Random|RandomFloatinRange 0.4 1.5))
            (if (< (Utilities|Array|Length (Variables|Default|GetAttackers)) (Variables|Default|GetMaxEnemiesAllowed))
              (CallFunction|SpawnAttackers)
              (goto _label)
              (else
                (goto _label)))))
        (:then_1
          (Audio|PlaySound2D "/Game/Sounds/AmbientNonLoops/Stereo/MetalCreak_Pillars01_Stereo.MetalCreak_Pillars01_Stereo" 1.0 1.0 0.0 0 0)
          (Utilities|FlowControl|Delay 2.5)
          (bind _returnvalue (Audio|SpawnSound2D "/Game/Sounds/Music/ShooterGame_Music_Cue.ShooterGame_Music_Cue" 1.0 1.0 0.0 0))
          (Variables|Default|SetGame%20Music _returnvalue))))))

(event Custom|Spawn%20Attackers
  (bind _outactors (Actor|GetAllActorsOfClass "/Game/Blueprints/Actors/EnemySpawner/BP_EnemySpawner.BP_EnemySpawner_C"))
  (bind _returnvalue (Game|SpawnActorfromClass "/Game/Blueprints/AI/AI_Attacker.AI_Attacker_C" (Math|Transform|MakeTransform (+ (Transformation|GetActorLocation (Utilities|Array|Get(acopy) _outactors (Math|Random|RandomIntegerinRange 0 (Utilities|Array|LastIndex _outactors)))) "0, 0,50.000000") "0, 0, 0" "1,1,1") "Undefined" 0 0))
  (Utilities|Array|Add (Variables|Default|GetAttackers) _returnvalue)
  (Math|Integer|DecrementInt (Variables|Default|GetEnemiesToSpawn)))

(event Custom|Wave%20Complete
  (Audio|Components|Audio|FadeOut (Variables|Default|GetGame%20Music) 2.0 0.0 :!class /Script/Engine.AudioComponent)
  (Utilities|FlowControl|Delay 3.0)
  (CallFunction|StartNewWave))

(event EventBeginPlay
  (Utilities|FlowControl|Delay 2.5)
  (CallFunction|StartNewWave))

(event EventTick
  (params (DeltaSeconds :type Float%20%28single-precision%29)))

(fn ConstructionScript)

(fn RemoveAttacker
  (params (Attacker :type AI%20Attacker%20Object%20Reference))
  (Utilities|Array|RemoveItem (Variables|Default|GetAttackers) Attacker)
  (if (== (Utilities|Array|Length (Variables|Default|GetAttackers)) 0)
    (CallFunction|WaveComplete)))